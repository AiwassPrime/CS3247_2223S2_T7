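; Behavior tree task for enemy AI that checks the controlled pawn's distance to the blackboard Target actor and writes the State key.
; It compares that distance to a fixed range threshold, but both branches write the same AttackState value, so the check has no effect on the result.
; It finishes with the Success variable, which it sets to false when Target is not a valid Actor.
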(event EventReceiveExecuteAI
  (params (OwnerController :type AI%20Controller%20Object%20Reference) (ControlledPawn :type Pawn%20Object%20Reference))
  (bind _asactor (Utilities|Casting|CastToActor (Class|BTFunctionLibrary|GetBlackboardValueasObject (Variables|Default|GetTarget)))
    (:then
      (if (<= (Transformation|GetDistanceTo ControlledPawn _asactor) 4e+02)
        (Class|BTFunctionLibrary|SetBlackboardValueasEnum (Variables|Default|GetState) (Variables|Default|GetAttackState))
        (else
          (Class|BTFunctionLibrary|SetBlackboardValueasEnum (Variables|Default|GetState) (Variables|Default|GetAttackState)))))
    (:CastFailed
      (Variables|Default|SetSuccess false)))
  (AI|BehaviorTree|FinishExecute (Variables|Default|GetSuccess)))
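; BP_Loot handles weighted random loot drops for the actor that owns it.
; DropLoot totals the weights in the LootTable map, then ChooseLoot rolls within that sum and subtracts each entry's weight until it lands on a key.
; The key drives a switch whose only case shown, 1, spawns a health potion at the owner's location, adjusted for collision.
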(event Custom|DropLoot
  (bind _sum (CallFunction|CalculateSum))
  (Variables|Default|SetValueSum _sum)
  (bind _loot (CallFunction|ChooseLoot))
  (switch int _loot
    (:1
      (Game|SpawnActorfromClass :Class "/Game/CS3247_2223S2_T7/Items/BP_Item1_HealthPotion.BP_Item1_HealthPotion_C" :SpawnTransform (Math|Transform|MakeTransform (Transformation|GetActorLocation (Components|GetOwner))) :CollisionHandlingOverride "AdjustIfPossibleButAlwaysSpawn" :Instigator 0))))

(event EventBeginPlay)

(event EventTick
  (params (DeltaSeconds :type Float%20%28single-precision%29)))

(fn CalculateSum
  (bind _values (Utilities|Map|Values (Variables|Default|GetLootTable)))
  (for _array_element _values
    (bind _output_get (LocalVariables|SetRunningTotal (+ (LocalVariables|GetRunningTotal) _array_element))))
  (return _output_get))

(fn ChooseLoot
  (LocalVariables|SetRandomValue (Math|Random|RandomFloatinRange 0.0 (Variables|Default|GetValueSum)))
  (bind _keys (Utilities|Map|Keys (Variables|Default|GetLootTable)))
  (for _array_element _keys
    (if (<= (LocalVariables|GetRandomValue) (.Value (Utilities|Map|Find (Variables|Default|GetLootTable) _array_element)))
      (return _array_element)
      (else
        (LocalVariables|SetRandomValue (- (LocalVariables|GetRandomValue) (.Value (Utilities|Map|Find (Variables|Default|GetLootTable) _array_element))))))))
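; BP_ky_darkStorm is a hero skill actor that damages enemies entering its Bx collision component.
; On overlap it reads ATK from the player's BP_HeroBase and calls HitOnce three times in immediate succession.
; HitOnce casts to each supported enemy class and calls HitEnemy without stun, giving Wolf and Sevarog a small fixed knockback and Crow none.
; The Attack function is an empty stub.
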(event OnComponentBeginOverlap(bx)
  (params (OverlappedComponent :type Primitive%20Component%20Object%20Reference) (OtherActor :type Actor%20Object%20Reference) (OtherComp :type Primitive%20Component%20Object%20Reference) (OtherBodyIndex :type Integer) (bFromSweep :type Boolean) (SweepResult :type Hit%20Result%20Structure%20%28by%20ref%29))
  (bind _asbp_hero_base (Utilities|Casting|CastToBP_HeroBase (Game|GetPlayerCharacter 0)))
  (Variables|Default|SetATK (Variables|/Game/CS3247_2223S2_T7/Hero/BP_HeroBase.BP_HeroBase_C|GetATK _asbp_hero_base))
  (CallFunction|HitOnce OtherActor)
  (CallFunction|HitOnce OtherActor)
  (CallFunction|HitOnce OtherActor))

(event Custom|Hit%20Once
  (params (Enemy :type Actor%20Object%20Reference))
  (bind _atk (Variables|Default|GetATK))
  (bind _asbp_wolf (Utilities|Casting|CastToBP_Wolf Enemy)
    (:then
      (Default|HitEnemy _asbp_wolf _atk "10.000000,10.000000,0.000000" false))
    (:CastFailed
      _))
  (bind _asbp_sevarog (Utilities|Casting|CastToBP_Sevarog Enemy)
    (:then
      (Default|HitEnemy _asbp_sevarog _atk "10.000000,10.000000, 0" false))
    (:CastFailed
      _))
  (bind _asbp_crow (Utilities|Casting|CastToBP_Crow Enemy))
  (Default|HitEnemy _asbp_crow _atk "0, 0, 0" false))

(event EventBeginPlay
  (|CallParentFunction) ; This node is disabled and will not be called.\nDrag off pins to build functionality.
)

(event Collision|EventActorBeginOverlap
  (params (OtherActor :type Actor%20Object%20Reference))
  (|CallParentFunction OtherActor) ; This node is disabled and will not be called.\nDrag off pins to build functionality.
)

(event EventTick
  (params (DeltaSeconds :type Float%20%28single-precision%29))
  (|CallParentFunction DeltaSeconds) ; This node is disabled and will not be called.\nDrag off pins to build functionality.
)

(fn ConstructionScript
  (|CallParentFunction))

(fn Attack)
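; Playable warrior hero with camera-relative movement, sword combos, a movement-locking block and cooldown heal and dark storm skills.
; Attacks cycle four montages and open a window where Box overlaps damage Wolf, Sevarog and Crow enemies.
; Tick caps HP, updates the HP widget, levels stats from Exp and handles death; GetHit subtracts guard from damage.
; The construction script links modular gear to the body mesh pose and toggles part visibility.
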(event OnComponentBeginOverlap(Box)
  (params (OverlappedComponent :type Primitive%20Component%20Object%20Reference) (OtherActor :type Actor%20Object%20Reference) (OtherComp :type Primitive%20Component%20Object%20Reference) (OtherBodyIndex :type Integer) (bFromSweep :type Boolean) (SweepResult :type Hit%20Result%20Structure%20%28by%20ref%29))
  (bind _atk (Variables|Default|GetATK))
  (if (Variables|Default|Getsword)
    (if (Variables|Default|GetMoveAb)
      (bind _asbp_wolf (Utilities|Casting|CastToBP_Wolf OtherActor)
        (:then
          (Game|SpawnActorfromClass "/Game/FXVarietyPack/Blueprints/BP_ky_hit1.BP_ky_hit1_C" (Math|Transform|MakeTransform (Transformation|GetWorldLocation (Variables|/Script/Engine.Actor|GetRootComponent _asbp_wolf)) "0, 0, 0" "0.300000,0.300000,0.300000") "Undefined" 0 0)
          (Default|HitEnemy _asbp_wolf _atk "10.000000,10.000000,0.000000" false))
        (:CastFailed
          _))
      (bind _asbp_sevarog (Utilities|Casting|CastToBP_Sevarog OtherActor)
        (:then
          (Game|SpawnActorfromClass "/Game/FXVarietyPack/Blueprints/BP_ky_hit1.BP_ky_hit1_C" (Math|Transform|MakeTransform (Transformation|GetWorldLocation (Variables|/Script/Engine.Actor|GetRootComponent _asbp_sevarog)) "0, 0, 0" "0.300000,0.300000,0.300000") "Undefined" 0 0)
          (Default|HitEnemy _asbp_sevarog _atk "10.000000,10.000000, 0" false))
        (:CastFailed
          _))
      (bind _asbp_crow (Utilities|Casting|CastToBP_Crow OtherActor))
      (Game|SpawnActorfromClass "/Game/FXVarietyPack/Blueprints/BP_ky_hit1.BP_ky_hit1_C" (Math|Transform|MakeTransform (Transformation|GetWorldLocation (Variables|/Script/Engine.Actor|GetRootComponent _asbp_crow)) "0, 0, 0" "0.300000,0.300000,0.300000") "Undefined" 0 0)
      (Default|HitEnemy _asbp_crow _atk "0, 0, 0" false))))

(event EventBeginPlay
  (|CallParentFunction)
  (Variables|Default|SetATK 35.0)
  (Variables|Default|SetHP 3e+02)
  (Variables|Default|SetHP_base 3e+02)
  (Variables|Default|SetExp 0.0)
  (Variables|Default|Setlevel 0)
  (Variables|Default|SetMoveAb true)
  (Variables|Default|Setsword false)
  (Variables|Default|SetGRD 3e+01)
  (Variables|Default|SetT_ready true)
  (Variables|Default|SetY_ready true)
  (Variables|Default|Setsp true))

(event Collision|EventActorBeginOverlap
  (params (OtherActor :type Actor%20Object%20Reference))
  (|CallParentFunction OtherActor))

(event EventTick
  (params (DeltaSeconds :type Float%20%28single-precision%29))
  (bind _returnvalue (Transformation|GetActorLocation))
  (|CallParentFunction DeltaSeconds)
  (if (>= (Variables|Default|GetHP_base) (Variables|Default|GetHP))
    _
    (else
      (Variables|Default|SetHP (Variables|Default|GetHP_base))))
  (if (>= 0.0 (Variables|Default|GetHP))
    (Widget|RemovefromParent (Variables|Default|GetHPRef))
    (Components|Movement|StopMovementImmediately (Variables|Character|GetCharacterMovement))
    (if (Variables|Default|Getsp)
      (Variables|Default|Setsp false)
      (Game|SpawnActorfromClass "/Game/FXVarietyPack/Blueprints/BP_ky_explosion.BP_ky_explosion_C" (Math|Conversions|ToTransform(Vector) _returnvalue) "Undefined" 0 0)
      (Audio|SpawnSoundatLocation "/Game/StarterContent/Audio/Collapse02.Collapse02" _returnvalue "0, 0, 0" 0.8 1.0 0.4 0 0)
      (Utilities|FlowControl|Delay 0.3)
      (Actor|DestroyActor)
      (bind _returnvalue_2 (Actor|GetActorOfClass "/Game/CS3247_2223S2_T7/Inventory/T_Character/BP_T_Character.BP_T_Character_C"))
      (Actor|DestroyActor _returnvalue_2))
    (else
      (CallFunction|UpdateHeroHp)
      (bind (_newlevel _up) (CallFunction|CheckUpgrade (Variables|Default|GetExp)))
      (if _up
        (bind _output_get (Variables|Default|Setlevel _newlevel))
        (Development|PrintString (Utilities|String|ToString(Integer) _output_get))
        (bind _output_get_2 (Variables|Default|SetATK (+ (Variables|Default|GetATK) 2e+01)))
        (Development|PrintString (Utilities|String|ToString(Float) _output_get_2))
        (bind _output_get_3 (Variables|Default|SetHP (+ 4e+01 (Variables|Default|GetHP))))
        (Development|PrintString (Utilities|String|ToString(Float) _output_get_3))
        (bind _output_get_4 (Variables|Default|SetHP_base (+ 4e+01 (Variables|Default|GetHP_base))))
        (Development|PrintString (Utilities|String|ToString(Float) _output_get_4))
        (bind _output_get_5 (Variables|Default|SetGRD (+ (Variables|Default|GetGRD) 1e+01)))
        (Development|PrintString (Utilities|String|ToString(Float) _output_get_5))))))

(event Input|ActionEvents|InputActionBlockHit
  (params (Key :type Key%20Structure :default "None"))
  (:Pressed
    (Components|Movement|StopMovementImmediately (Variables|Character|GetCharacterMovement))
    (Animation|Montage|PlayMontage (Variables|Character|GetMesh) 0
      (:then
        (Variables|Default|SetMoveAb false))))
  (:Released
    (Animation|StopAnimMontage 0)
    (Variables|Default|SetMoveAb true)))

(event Input|ActionEvents|InputActionSwordAttack
  (params (Key :type Key%20Structure :default "None"))
  (:Pressed
    (Variables|Default|Setsword true)
    (if (not (Variables|Default|GetIsAttacking))
      (Variables|Default|SetIsAttacking true)
      ;[1 1 1] Attack
      (Animation|PlayAnimMontage (Utilities|Select :Index (Math|Integer|%(Integer) (Variables|Default|GetAttack%20Count) 4) :Option%200 "/Game/WarriorHero/Animations/Anim_Attack_Right_Shield_Montage.Anim_Attack_Right_Shield_Montage" :Option%201 "/Game/WarriorHero/Animations/Anim_Attack_Left_Shield_Montage.Anim_Attack_Left_Shield_Montage" :Option%202 "/Game/WarriorHero/Animations/Anim_Attack_Shield_Montage.Anim_Attack_Shield_Montage" :Option%203 "/Game/WarriorHero/Animations/Anim_Attack_Top_Shield_Montage.Anim_Attack_Top_Shield_Montage") 1.5 "Default")
      (Math|Integer|IncrementInt (Variables|Default|GetAttack%20Count)
        (:%20%20
          (Utilities|FlowControl|Delay 0.7)
          (Variables|Default|SetIsAttacking false)
          (Variables|Default|Setsword false))))))

(event Input|AxisEvents|InputAxisMoveForward
  (params (AxisValue :type Float%20%28single-precision%29))
  (if (Variables|Default|GetMoveAb)
    (Pawn|Input|AddMovementInput (Math|Vector|GetForwardVector (Math|Rotator|MakeRotator 0.0 0.0 (.Yaw (Math|Rotator|BreakRotator (Pawn|GetControlRotation :!class /Script/Engine.Pawn))))) AxisValue false)))

(event Input|AxisEvents|InputAxisMoveRight
  (params (AxisValue :type Float%20%28single-precision%29))
  (if (Variables|Default|GetMoveAb)
    (Pawn|Input|AddMovementInput (Math|Vector|GetRightVector (Math|Rotator|MakeRotator 0.0 0.0 (.Yaw (Math|Rotator|BreakRotator (Pawn|GetControlRotation :!class /Script/Engine.Pawn))))) AxisValue false)))

(event Input|KeyboardEvents|T
  (params (Key :type Key%20Structure :default "None"))
  (bind _returnvalue (Transformation|GetActorRotation))
  (bind _returnvalue_2 (Transformation|GetActorLocation))
  (bind _returnvalue_3 (Math|Vector|GetForwardVector _returnvalue))
  (:Pressed
    (if (Variables|Default|GetT_ready)
      (Variables|Default|SetT_ready false)
      (Game|SpawnActorfromClass "/Game/FXVarietyPack/Blueprints/BP_ky_darkStorm.BP_ky_darkStorm_C" (Math|Conversions|ToTransform(Vector) (+ (Math|Vector|MakeVector (.x _returnvalue_2) (.y _returnvalue_2) 1.5e+02) (Math|Vector|MakeVector (* 400 (.x _returnvalue_3)) (* 400 (.y _returnvalue_3)) 0.0))) "AlwaysSpawn" 0 0)
      (Utilities|FlowControl|Delay 3.0)
      (Variables|Default|SetT_ready true))))

(event Input|KeyboardEvents|Y
  (params (Key :type Key%20Structure :default "None"))
  (:Pressed
    (if (Variables|Default|GetY_ready)
      (Variables|Default|SetY_ready false)
      (Game|SpawnActorfromClass "/Game/FXVarietyPack/Blueprints/BP_ky_healAura.BP_ky_healAura_C" (Math|Transform|MakeTransform (+ (* (Transformation|GetActorLocation) "1.000000,1.000000,0.000000") "0, 0,50.000000") "0, 0, 0" "2.000000,2.000000,2.000000") "Undefined" 0 0)
      (bind _output_get (Variables|Default|SetHP (+ (Variables|Default|GetHP) 15.0)))
      (Development|PrintString (Utilities|String|ToString(Float) _output_get))
      (Utilities|FlowControl|Delay 5.0)
      (Variables|Default|SetY_ready true))))

(fn ConstructionScript
  (Class|SkinnedMeshComponent|SetMasterPoseComponent (Variables|Default|GetLegArmor) (Variables|Character|GetMesh) false)
  (Utilities|FlowControl|Sequence
    (:then_0
      (Rendering|SetVisibility (Variables|Default|GetBeard) (Variables|Customisation|GetBeardVisibility) false))
    (:then_1
      (Rendering|SetVisibility (Variables|Default|GetBodyArmor) (Variables|Customisation|GetBodyArmorVisibility) false))
    (:then_2
      (Rendering|SetVisibility (Variables|Default|GetArmArmor) (Variables|Customisation|GetArmArmorVisibility) false))
    (:then_3
      (Rendering|SetVisibility (Variables|Default|GetLegArmor) (Variables|Customisation|GetLegArmorVisibility) false))
    (:then_4
      (Rendering|SetVisibility (Variables|Default|GetBeltBag) (Variables|Customisation|GetBeltBagVisibility) false))
    (:then_5
      (Rendering|SetVisibility (Variables|Default|GetShield) (Variables|Customisation|GetShieldVisibility) false))
    (:then_6
      (Rendering|SetVisibility (Variables|Default|GetSM_Sword) (Variables|Customisation|GetSwordVisibility) false))))

(fn UpdateHeroHp
  (Variables|/Game/CS3247_2223S2_T7/Hero/WarriorHero/Blueprint/BP_HeroHealthBar.BP_HeroHealthBar_C|SetHeroHP (Variables|Default|GetHPRef) (/ (Variables|Default|GetHP) (Variables|Default|GetHP_base)))
  (return))

(fn UpdateHeroExp
  (params (exp_get :type Float%20%28single-precision%29))
  (Variables|Default|SetExp (+ (Variables|Default|GetExp) exp_get))
  (return))

(fn CheckUpgrade
  (params (exp :type Float%20%28single-precision%29))
  (bind _returnvalue (/ exp 1e+02))
  (bind _returnvalue_2 (Math|Float|Truncate _returnvalue))
  (return _returnvalue_2 (> _returnvalue_2 (Variables|Default|Getlevel))))

(fn GetHit
  (params (Damage :type Float%20%28single-precision%29))
  (bind _grd (Variables|Default|GetGRD))
  (if (> (- Damage _grd) 0.0)
    (Variables|Default|SetHP (+ (- (Variables|Default|GetHP) Damage) _grd))
    (Audio|PlaySoundatLocation "/Game/CS3247_2223S2_T7/Hero/WarriorHero/Blueprint/bp_herogethit.bp_herogethit" (Transformation|GetActorLocation) "0, 0, 0" 1.0 1.0 0.0 0 0 0)
    (return 0)))
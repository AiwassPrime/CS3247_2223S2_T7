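; BP_MockPlayer is a mock player for testing enemies, with basic movement, look and debug attack inputs.
; Axis inputs move it on the horizontal plane relative to control yaw and drive controller yaw and pitch.
; TestAttack sends a fixed-damage HitEnemy through BPI_Enemies to Characters in the level regardless of range, printing a confirmation.
; TestTriggerAttack makes every BP_Wolf perform its MeleeAttack.
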(event EventBeginPlay)

(event Collision|EventActorBeginOverlap
  (params (OtherActor :type Actor%20Object%20Reference)))

(event EventTick
  (params (DeltaSeconds :type Float%20%28single-precision%29)))

(event Input|ActionEvents|InputActionTestAttack
  (params (Key :type Key%20Structure :default "None"))
  (:Pressed
    (bind _outactors (Actor|GetAllActorsOfClass "/Script/Engine.Character"))
    (for _array_element _outactors
      (bind _asbpi_enemies (Utilities|Casting|CastToBPI_Enemies _array_element))
      (Default|HitEnemy _asbpi_enemies 2e+01 "0, 0, 0" false)
      (Development|PrintString "Test hit: dmg = 20"))))

(event Input|ActionEvents|InputActionTestTriggerAttack
  (params (Key :type Key%20Structure :default "None"))
  (:Pressed
    (bind _outactors (Actor|GetAllActorsOfClass "/Game/CS3247_2223S2_T7/Enemies/Wolf/BP_Wolf.BP_Wolf_C"))
    (for _array_element _outactors
      (Default|MeleeAttack _array_element))))

(event Input|AxisEvents|InputAxisLookUp
  (params (AxisValue :type Float%20%28single-precision%29))
  (Pawn|Input|AddControllerPitchInput AxisValue))

(event Input|AxisEvents|InputAxisTurn
  (params (AxisValue :type Float%20%28single-precision%29))
  (Pawn|Input|AddControllerYawInput AxisValue))

(event Input|AxisEvents|InputAxisMoveForward
  (params (AxisValue :type Float%20%28single-precision%29))
  (Pawn|Input|AddMovementInput (Math|Vector|GetForwardVector (Math|Rotator|MakeRotator 0.0 0.0 (.Yaw (Math|Rotator|BreakRotator (Pawn|GetControlRotation :!class /Script/Engine.Pawn))))) AxisValue false))

(event Input|AxisEvents|InputAxisMoveRight
  (params (AxisValue :type Float%20%28single-precision%29))
  (Pawn|Input|AddMovementInput (Math|Vector|GetRightVector (Math|Rotator|MakeRotator 0.0 0.0 (.Yaw (Math|Rotator|BreakRotator (Pawn|GetControlRotation :!class /Script/Engine.Pawn))))) AxisValue false))

(fn ConstructionScript)